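; OnlinePlayerState is a player state Blueprint that tracks one player's kills and personal score.
; GainKill increments the kill count and fires the OnKillEarned dispatcher with the player and the victim.
; GainScore adds to the personal score, then forwards the points with the player's ID to AddPlayerPoint on OnlineGameState.
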(event Custom|GainKill
  (params (Victim :type String))
  (Variables|Default|SetKills (+ (Variables|Default|GetKills) 1))
  (Default|CallOnKillEarned self Victim))

(event Custom|GainScore
  (params (Score :type Integer))
  (Variables|Default|SetPersonalScore (+ Score (Variables|Default|GetPersonalScore)))
  (bind _asonline_game_state (Utilities|Casting|CastToOnlineGameState (Game|GetGameState)))
  (Default|AddPlayerPoint _asonline_game_state (Variables|Default|GetPlayerId) Score))

(fn ConstructionScript)