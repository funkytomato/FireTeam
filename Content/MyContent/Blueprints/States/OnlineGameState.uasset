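; Game state for online matches that tracks player and team scores and announces kills.
; New players' kill-earned events are bound on join, and AnnounceKill relays to an RPC that adds a killer/victim widget to the local HUD's announcement tray.
; Point events update scoreboard maps and broadcast both through OnScoreUpdated, though team scoring always reads team 0's total before adding.
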(event Custom|AnnounceKill
  (params (Killer :type Player%20State%20Object%20Reference) (Victim :type String))
  (CallFunction|RPCKillAnnounced Killer Victim))

(event Custom|RPC_KillAnnounced
  (params (Killer :type Player%20State%20Object%20Reference) (Victim :type String))
  (bind _returnvalue (UserInterface|CreateWidget "/Game/MyContent/UI/KillAnnouncement_WBP.KillAnnouncement_WBP_C" 0 (PlayerState|GetPlayerName Killer) Victim))
  (bind _asin_game_hud (Utilities|Casting|CastToInGameHUD (HUD|GetHUD (Game|GetPlayerController 0))))
  (Default|AddAnnoucement (Variables|/Game/MyContent/UI/PlayerInGameHUD_WBP.PlayerInGameHUD_WBP_C|GetAnnouncementTray_WBP (Variables|/Game/MyContent/UI/InGameHUD.InGameHUD_C|GetInGameHUD _asin_game_hud)) _returnvalue))

(event Custom|NewPlayerJoined
  (params (Controller :type Player%20Controller%20Object%20Reference))
  (EventDispatchers|BindEventtoOnKillEarned (.AsOnline%20Player%20State (Utilities|Casting|CastToOnlinePlayerState (Variables|/Script/Engine.Controller|GetPlayerState Controller))) (EventDispatchers|CreateEvent :!event Custom|AnnounceKill)))

(event Custom|AddPlayerPoint
  (params (PlayerID :type Integer) (Score :type Integer))
  (bind _playerscoreboard (Variables|Default|GetPlayerScoreboard))
  (Utilities|Map|Add _playerscoreboard PlayerID (+ Score (.Value (Utilities|Map|Find _playerscoreboard PlayerID))))
  (Default|CallOnScoreUpdated (Variables|Default|GetPlayerScoreboard) (Variables|Default|GetTeamScoreboard)))

(event Custom|AddTeamPoint
  (params (TeamId :type Integer) (Score :type Integer))
  (bind _teamscoreboard (Variables|Default|GetTeamScoreboard))
  (Utilities|Map|Add _teamscoreboard TeamId (+ Score (.Value (Utilities|Map|Find _teamscoreboard 0))))
  (Default|CallOnScoreUpdated (Variables|Default|GetPlayerScoreboard) (Variables|Default|GetTeamScoreboard)))

(fn ConstructionScript)