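; Game mode for online matches that handles player joins, respawns and score-based win detection.
; Login and controller-swap events register players with OnlineGameState, while Respawn destroys the controller's pawn and restarts the player.
; ReadyToEndMatch scans the game state's team or player scoreboard, chosen by IsTeamType, ending the match when a score reaches WinThreshold and recording the winning team or player ID.
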(event Custom|Respawn
  (params (Controller :type Player%20Controller%20Object%20Reference))
  (Actor|DestroyActor (Pawn|GetControlledPawn Controller))
  (Utilities|IsValid Controller
    (:Is%20Valid
      (Class|GameModeBase|RestartPlayer Controller))))

(event EventPostLogin
  (params (NewPlayer :type Player%20Controller%20Object%20Reference))
  (bind _asonline_game_state (Utilities|Casting|CastToOnlineGameState (Game|GetGameState)))
  (Default|NewPlayerJoined _asonline_game_state NewPlayer))

(event EventOnSwapPlayerControllers
  (params (OldPC :type Player%20Controller%20Object%20Reference) (NewPC :type Player%20Controller%20Object%20Reference))
  (bind _asonline_game_state (Utilities|Casting|CastToOnlineGameState (Game|GetGameState)))
  (Default|NewPlayerJoined _asonline_game_state NewPC))

(fn ConstructionScript)

(fn ReadytoEndMatch
  (bind _asonline_game_state (Utilities|Casting|CastToOnlineGameState (Game|GetGameState)))
  (bind _keys (Utilities|Map|Keys (select (Variables|Default|GetIsTeamType) (Variables|/Game/MyContent/Blueprints/States/OnlineGameState.OnlineGameState_C|GetTeamScoreboard _asonline_game_state) (Variables|/Game/MyContent/Blueprints/States/OnlineGameState.OnlineGameState_C|GetPlayerScoreboard _asonline_game_state))))
  (for _array_element _keys
    (if (>= (.Value (Utilities|Map|Find (select (Variables|Default|GetIsTeamType) (Variables|/Game/MyContent/Blueprints/States/OnlineGameState.OnlineGameState_C|GetTeamScoreboard _asonline_game_state) (Variables|/Game/MyContent/Blueprints/States/OnlineGameState.OnlineGameState_C|GetPlayerScoreboard _asonline_game_state)) _array_element)) (Variables|Default|GetWinThreshold))
      (Variables|Default|SetWinningPlayerID (Math|Integer|SelectInt -1 _array_element (Variables|Default|GetIsTeamType)))
      (Variables|Default|SetWinningTeamID (Math|Integer|SelectInt _array_element -1 (Variables|Default|GetIsTeamType)))
      (return true)))
  (return false))