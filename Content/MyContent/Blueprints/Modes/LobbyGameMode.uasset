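; LobbyGameMode is a lobby game mode that tracks connected players and shares the player list with their controllers.
; On PostLogin, it stores each LobbyController and gives it a player info struct with the PlayerState name and default level and ready state.
; It appends that info to a shared array, then calls UpdatePlayerList on every connected controller with the full list.
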(event EventPostLogin
  (params (NewPlayer :type Player%20Controller%20Object%20Reference))
  (bind _aslobby_controller (Utilities|Casting|CastToLobbyController NewPlayer))
  (Utilities|Array|Add (Variables|Default|GetConnectedPlayers) _aslobby_controller)
  (bind _output_get (Variables|/Game/MyContent/Menu/LobbyController.LobbyController_C|SetPlayerInfo _aslobby_controller (Utilities|Struct|MakePlayerInfo (PlayerState|GetPlayerName (Variables|/Script/Engine.Controller|GetPlayerState NewPlayer)) 0 false)))
  (Utilities|Array|Add (Variables|Default|GetConnectedPlayerInfo) _output_get)
  (for _array_element (Variables|Default|GetConnectedPlayers)
    (Default|UpdatePlayerList _array_element (Variables|Default|GetConnectedPlayerInfo))))

(fn ConstructionScript)