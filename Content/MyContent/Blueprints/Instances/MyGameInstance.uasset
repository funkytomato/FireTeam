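; Game instance that handles LAN multiplayer sessions: hosting, searching, joining and quick match.
; Hosting creates a session and opens LobbyMenu as a listen server; FindMatch broadcasts results through OnSessionsFound, while SearchSessions stores them in FoundSessions.
; QuickMatch joins the first search result, hosting only if the search fails.
; JoinSessionByIndex rejects index 0 and indexes FoundSessions by its length, not the given index.
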(event Custom|QuickMatch
  (bind _results (|FindSessions (Game|GetPlayerController 0) 10 true)
    (:OnSuccess
      (|JoinSession (Game|GetPlayerController 0) (Utilities|Array|Get(acopy) _results)
        (:OnSuccess
          (Development|PrintString "Successfully joined Session"))
        (:OnFailure
          (Development|PrintString "Failed to join Session"))))
    (:OnFailure
      (CallFunction|HostMatch))))

(event Custom|HostMatch
  (|Session (Game|GetPlayerController 0) 8 true
    (:OnSuccess
      (Development|PrintString "Success hosting session")
      (Game|OpenLevel(byObjectReference) "/Game/MyContent/Menu/LobbyMenu.LobbyMenu" true "?listen"))
    (:OnFailure
      (Development|PrintString "Failed to host match"))))

(event Custom|FindMatch
  (bind _results (|FindSessions (Game|GetPlayerController 0) 10 true)
    (:OnSuccess
      (Development|PrintString "Session found")
      (Default|CallOnSessionsFound _results))
    (:OnFailure
      (Development|PrintString "Failed to find Session"))))

(event Custom|SearchSessions
  (bind _results (|FindSessions (Game|GetPlayerController 0) 15 true)
    (:OnSuccess
      (Variables|Default|SetFoundSessions _results))))

(event Custom|JoinSessionByIndex
  (params (SessionIndex :type Integer%20%28by%20ref%29))
  (bind _foundsessions (Variables|Default|GetFoundSessions))
  (bind _returnvalue (Utilities|Array|Length _foundsessions))
  (if (and (> SessionIndex 0) (< SessionIndex _returnvalue))
    (bind _asmy_game_instance (Utilities|Casting|CastToMyGameInstance (Game|GetGameInstance)))
    (CallFunction|JoinSession _asmy_game_instance (Utilities|Array|Get(acopy) (Variables|Default|GetFoundSessions) _returnvalue))))

(event Custom|JoinSession
  (params (SearchResult :type Blueprint%20Session%20Result%20Structure%20%28by%20ref%29))
  (|JoinSession (Game|GetPlayerController 0) SearchResult
    (:OnSuccess
      (Development|PrintString "Successfully joined Session"))
    (:OnFailure
      (Development|PrintString "Failed to join Session"))))